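; BlueDoor is a door actor that opens only when the player character has collected the blue coin.
; On BeginPlay it caches the player's BP_ThirdPersonCharacter.
; Any actor overlap checks that character's BlueCoinCollected flag, without checking which actor overlapped.
; If set, it clears the flag, prints a message and destroys the door; otherwise it prints that the coin is missing.
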(event `self.ReceiveBeginPlay`
  (bind _asbp_third_person_character (cast `/Game/ThirdPerson/Blueprints/BP_ThirdPersonCharacter` (`GameplayStatics.GetPlayerCharacter` 0)))
  (set `self.Character REF` _asbp_third_person_character))

(event `self.ReceiveActorBeginOverlap`
  (params (OtherActor :type "Actor Object Reference"))
  (if (`/Game/ThirdPerson/Blueprints/BP_ThirdPersonCharacter.Blue_Coin_Collected` (`self.Character REF`))
    (set `/Game/ThirdPerson/Blueprints/BP_ThirdPersonCharacter.Blue_Coin_Collected` false (`self.Character REF`))
    (`KismetSystemLibrary.PrintText` "Door Open")
    (`self.K2_DestroyActor`)
    (else
      (`KismetSystemLibrary.PrintText` "Missing Coin"))))

(fn `UserConstructionScript`)